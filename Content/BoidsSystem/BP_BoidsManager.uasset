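; BP_BoidsManager spawns the initial population of BP_Boids actors for the boids system.
; On BeginPlay it loops Count times, giving each boid a random location in a box around the world origin, random pitch and yaw, and a random non-uniform scale.
; Spawns ignore collisions, and the manager keeps no references to the boids or any logic to update them afterwards.
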(event `self.ReceiveBeginPlay`
  (bind _returnvalue (`KismetMathLibrary.RandomFloatInRange` 0.5 1.0))
  (bind _returnvalue_2 (`KismetMathLibrary.RandomFloatInRange` -180.0 180.0))
  (for _ (range 1 (+ (`self.Count`) 1))
    (`|SpawnActorFromClass` "/Game/BoidsSystem/BP_Boids.BP_Boids_C" (`KismetMathLibrary.MakeTransform` (`KismetMathLibrary.MakeVector` (`KismetMathLibrary.RandomFloatInRange` -500.0 500.0) (`KismetMathLibrary.RandomFloatInRange` -500.0 500.0) (`KismetMathLibrary.RandomFloatInRange` -800.0 800.0)) (`KismetMathLibrary.MakeRotator` 0.0 _returnvalue_2 _returnvalue_2) (`KismetMathLibrary.MakeVector` _returnvalue _returnvalue _returnvalue)) "AlwaysSpawn" "MultiplyWithRoot" null null)))

(fn `UserConstructionScript`)