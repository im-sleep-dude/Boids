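; Boid actor, apparently a fish, that flocks with other BP_Boids inside a BP_BoidsAreaBox.
; Two overlap spheres maintain neighbor lists that feed alignment, separation and cohesion offsets applied on Tick.
; Non-leaders follow and match a random leader chosen at BeginPlay; boids without leaders move forward, with timer-randomized rotation targets.
; A timeline turns strays back toward the box, and a sphere trace triggers a temporary dodge from static objects.
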(event `MoveBehindLeader`
  ; الايفينت بتاع المش ورا القائد لغير القائد
  (`self.K2_AddActorWorldOffset` (* (* (`KismetMathLibrary.Normal` (- (- (`self.K2_GetActorLocation` (`self.AssignedLeader`)) (`self.K2_GetActorLocation`)) (`KismetMathLibrary.RandomFloatInRange` 30.0 60.0))) 200.0) (stale `self.ReceiveTick` DeltaSeconds))))

(event `self.ReceiveTick`
  (params (DeltaSeconds :type "Float (single-precision)"))
  (bind (_returnvalue_roll _returnvalue_pitch _returnvalue_yaw) (`KismetMathLibrary.BreakRotator` (`self.K2_GetActorRotation`)))
  (bind (_returnvalue_roll_2 _returnvalue_pitch_2 _returnvalue_yaw_2) (`KismetMathLibrary.BreakRotator` (`self.K2_GetActorRotation`)))
  (bind (_returnvalue_roll_3 _returnvalue_pitch_3 _returnvalue_yaw_3) (`KismetMathLibrary.BreakRotator` (`self.K2_GetActorRotation`)))
  (bind _fishareabox_ref (`self.FishAreaBox_REF`))
  (bind _returnvalue (`SceneComponent.K2_GetComponentLocation` (`self.Mesh`)))
  (bind (_returnvalue_roll_4 _returnvalue_pitch_4 _returnvalue_yaw_4) (`KismetMathLibrary.BreakRotator` (`KismetMathLibrary.FindLookAtRotation` (`self.K2_GetActorLocation`) (`SceneComponent.K2_GetComponentLocation` (`/Game/BoidsSystem/BP_BoidsAreaBox.Box` _fishareabox_ref)))))
  (`|ExecutionSequence`
    (:`then_0`
      ; الكون هيميل لنفس اتجاه اللي حواليه
      (if (or (not (`self.DodgingBlocker`)) (not (`self.IsBack?`)) (`self.Alignment?`))
        (if (not (`self.CloseExist?`))
          (set `self.AlignmentVector ` (0.0 0.0 0.0))
          (for _array_element (`self.Neighbors`)
            (set `self.AlignmentVector ` (+ (`KismetMathLibrary.GetForwardVector` (`self.K2_GetActorRotation` _array_element)) (`self.AlignmentVector `))))
          (`self.K2_AddActorWorldOffset` (* (* (* (`KismetMathLibrary.Normal` (`self.AlignmentVector `)) (`self.AlignmentValue`)) 300.0) DeltaSeconds)))))
    (:`then_1`
      ; كل كون يبعد عن القريب منه عشان ميغبطوش ف بعض
      (if (and (`self.Separation?`) (not (`self.DodgingBlocker`)))
        (set `self.SeparationVector` (0.0 0.0 0.0))
        (for _array_element_2 (`self.CloseNeighbors`)
          (set `self.SeparationVector` (+ (`KismetMathLibrary.Normal` (- (`self.K2_GetActorLocation`) (`self.K2_GetActorLocation` _array_element_2))) (`self.SeparationVector`))))
        (`self.K2_AddActorWorldOffset` (* (* (* (`self.SeparationVector`) 100.0) DeltaSeconds) (`self.SeparationValue`)))))
    (:`then_2`
      ; المشي عادي و المشي ورا القائد
      (if (> (`KismetArrayLibrary.Array_Length` (`self.Leaders`)) 0)
        (if (not (`self.IsLeader?`))
          (if (not (`self.DodgingBlocker`))
            (`self.MoveBehindLeader`)))
        (else
          (`self.K2_AddActorWorldOffset` (* (* (`self.GetActorForwardVector`) (`self.Speed`)) DeltaSeconds)))))
    (:`then_3`
      ; بيغير اتجاه الحركة
      (if (not (`self.IsBack?`))
        (`self.K2_SetActorRotation` (`KismetMathLibrary.MakeRotator` (`KismetMathLibrary.FInterpTo` _returnvalue_roll_3 (`self.Value`) DeltaSeconds 1.0) (`KismetMathLibrary.FInterpTo` _returnvalue_pitch_3 (`self.Value`) DeltaSeconds 1.0) (`KismetMathLibrary.FInterpTo` _returnvalue_yaw_3 (`self.Value`) DeltaSeconds 1.0)))))
    (:`then_4`
      ; ميطلعش بره البوكس كولليجن ولو طلع يرجعله
      (if (`KismetMathLibrary.IsPointInBoxWithTransform` (`self.K2_GetActorLocation`) (`self.GetTransform` _fishareabox_ref) (1500.0 1500.0 1500.0))
        (set `self.IsBack?` false)
        (elif (not (`self.DodgingBlocker`))
          (set `self.IsBack?` true)
          (bind (_direction _alpha) (`Timeline|Timeline` :!label _label)
            (:`Update`
              (bind (_returnvalue_roll_5 _returnvalue_pitch_5 _returnvalue_yaw_5) (`KismetMathLibrary.BreakRotator` (`KismetMathLibrary.RLerp` (`KismetMathLibrary.MakeRotator` 0.0 _returnvalue_pitch _returnvalue_yaw) (`KismetMathLibrary.MakeRotator` 0.0 _returnvalue_pitch_4 _returnvalue_yaw_4) _alpha true)))
              (`self.K2_SetActorRotation` (`KismetMathLibrary.MakeRotator` 0.0 _returnvalue_pitch_5 _returnvalue_yaw_5)))
            (:`Finished`
              (`self.Reset`))))))
    (:`then_5`
      ; يبعد عن اي ستاتيك ميش في الماب
      (if (`self.AvoidStaticMesh?`)
        (bind (_outhit _returnvalue_2) (`KismetSystemLibrary.SphereTraceSingleForObjects` _returnvalue _returnvalue 400.0 (`|MakeArray` "ObjectTypeQuery1" :!type "EObjectTypeQuery Enum")))
        (if _returnvalue_2
          (set `self.DodgingBlocker` true)
          (bind (_returnvalue_roll_6 _returnvalue_pitch_6 _returnvalue_yaw_6) (`KismetMathLibrary.BreakRotator` (`KismetMathLibrary.Conv_VectorToRotator` (+ (`self.GetActorForwardVector`) (`.ImpactPoint` (`GameplayStatics.BreakHitResult` _outhit))))))
          (`self.K2_SetActorRotation` (`KismetMathLibrary.MakeRotator` 0.0 (`KismetMathLibrary.FInterpTo` _returnvalue_pitch_2 _returnvalue_pitch_6 DeltaSeconds 5.0) (`KismetMathLibrary.FInterpTo` _returnvalue_yaw_2 _returnvalue_yaw_6 DeltaSeconds 5.0)))
          (`KismetSystemLibrary.Delay` 2.0)
          (set `self.DodgingBlocker` false))))
    (:`then_6`
      ; التابع يلف زي ما القائد بيلف
      (if (> (`KismetArrayLibrary.Array_Length` (`self.Leaders`)) 0)
        (if (`self.IsLeader?`)
          _
          (elif (not (`self.DodgingBlocker`))
            (`self.K2_SetActorRotation` (`KismetMathLibrary.RInterpTo` (`self.K2_GetActorRotation`) (`self.K2_GetActorRotation` (`self.AssignedLeader`)) DeltaSeconds 5.0))))))
    (:`then_7`
      ; بيجمع الجيران في منطقطة مع بعض
      (if (and (`self.Cohesion?`) (not (`self.DodgingBlocker`)))
        (set `self.Count` 0)
        (set `self.SumLocations` (0.0 0.0 0.0))
        (for _array_element_3 (`self.Neighbors`)
          (set `self.SumLocations` (+ (`self.K2_GetActorLocation` _array_element_3) (`self.SumLocations`)))
          (`/Engine/EditorBlueprintResources/StandardMacros.IncrementInt` (`self.Count`)))
        (if (> (`KismetArrayLibrary.Array_Length` (`self.Neighbors`)) 0)
          (if (not (< (`self.Count`) 0))
            (`self.K2_AddActorWorldOffset` (* (* (* (`KismetMathLibrary.Normal` (- (/ (`self.SumLocations`) (`self.Count`)) (`self.K2_GetActorLocation`))) 250.0) DeltaSeconds) (`self.CohesionValue`)))))))))

(event `Reset`
  ; ميطلعش بره البوكس كولليجن ولو طلع يرجعله
  (goto _label :!via `SetNewTime`))

(event `self.ReceiveBeginPlay`
  (bind _returnvalue (`KismetArrayLibrary.Array_Length` (`self.Leaders`)))
  ; بيغير القيمة بتاعت الاتجاه كل كام ثانية
  (`|ExecutionSequence`
    (:`then_0`
      (bind _returnvalue_2 (`GameplayStatics.GetActorOfClass` "/Game/BoidsSystem/BP_BoidsAreaBox.BP_BoidsAreaBox_C"))
      (set `self.FishAreaBox_REF` _returnvalue_2))
    (:`then_1`
      (`KismetSystemLibrary.K2_SetTimerDelegate` (delegate `ChangeDircetionValue`) (`KismetMathLibrary.RandomFloatInRange` 1.0 3.0) true))
    (:`then_2`
      (if (not (`self.IsLeader?`))
        ; التابع بيختار ليدر
        (bind _outactors (`GameplayStatics.GetAllActorsOfClass` "BP_Boids_C"))
        (for _array_element _outactors
          (if (`/Game/BoidsSystem/BP_Boids.IsLeader?` _array_element)
            (`KismetArrayLibrary.Array_Add` (`self.Leaders`) _array_element)))
        (if (> _returnvalue 0)
          (set `self.AssignedLeader` (`|GetArrayItem` (`self.Leaders`) (`KismetMathLibrary.RandomIntegerInRange` 0 (- _returnvalue 1)))))))))

(event `ChangeDircetionValue`
  ; بيغير القيمة بتاعت الاتجاه كل كام ثانية
  (set `self.Value` (`KismetMathLibrary.RandomFloatInRange` -180.0 180.0)))

(event `self.NeighborSphere.OnComponentBeginOverlap`
  (params (OverlappedComponent :type "PrimitiveComponent Object Reference") (OtherActor :type "Actor Object Reference") (OtherComp :type "PrimitiveComponent Object Reference") (OtherBodyIndex :type Integer) (bFromSweep :type Boolean) (SweepResult :type "HitResult Structure (by ref)"))
  ; بيحط الجيران في ارراي ولو طلعوا من السفير بتاعته يمسحهم من الارراي
  (bind _asbp_boids (cast `/Game/BoidsSystem/BP_Boids` OtherActor))
  (if (!= OtherActor self)
    (`KismetArrayLibrary.Array_Add` (`self.Neighbors`) _asbp_boids)
    (set `/Game/BoidsSystem/BP_Boids.CloseExist?` true _asbp_boids)))

(event `self.NeighborSphere.OnComponentEndOverlap`
  (params (OverlappedComponent :type "PrimitiveComponent Object Reference") (OtherActor :type "Actor Object Reference") (OtherComp :type "PrimitiveComponent Object Reference") (OtherBodyIndex :type Integer))
  ; بيحط الجيران في ارراي ولو طلعوا من السفير بتاعته يمسحهم من الارراي
  (bind _asbp_boids (cast `/Game/BoidsSystem/BP_Boids` OtherActor))
  (`KismetArrayLibrary.Array_RemoveItem` (`self.Neighbors`) _asbp_boids)
  (set `/Game/BoidsSystem/BP_Boids.CloseExist?` false _asbp_boids))

(event `self.SeparationSphere.OnComponentBeginOverlap`
  (params (OverlappedComponent :type "PrimitiveComponent Object Reference") (OtherActor :type "Actor Object Reference") (OtherComp :type "PrimitiveComponent Object Reference") (OtherBodyIndex :type Integer) (bFromSweep :type Boolean) (SweepResult :type "HitResult Structure (by ref)"))
  ; بيحط الجيران في ارراي ولو طلعوا من السفير بتاعته يمسحهم من الارراي  بس دي سفير صغيرة
  (bind _asbp_boids (cast `/Game/BoidsSystem/BP_Boids` OtherActor))
  (if (!= OtherActor self)
    (`KismetArrayLibrary.Array_Add` (`self.CloseNeighbors`) _asbp_boids)))

(event `self.SeparationSphere.OnComponentEndOverlap`
  (params (OverlappedComponent :type "PrimitiveComponent Object Reference") (OtherActor :type "Actor Object Reference") (OtherComp :type "PrimitiveComponent Object Reference") (OtherBodyIndex :type Integer))
  ; بيحط الجيران في ارراي ولو طلعوا من السفير بتاعته يمسحهم من الارراي  بس دي سفير صغيرة
  (bind _asbp_boids (cast `/Game/BoidsSystem/BP_Boids` OtherActor))
  (`KismetArrayLibrary.Array_RemoveItem` (`self.CloseNeighbors`) _asbp_boids))

(fn `UserConstructionScript`
  (`SphereComponent.SetSphereRadius` (`self.NeighborSphere`) (`self.NeighborSphereRadius`) true)
  (`SphereComponent.SetSphereRadius` (`self.SeparationSphere`) (`self.SeparationSphereRadius`) true))